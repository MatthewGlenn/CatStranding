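; Asteroid actor with a Paper2D sprite and capsule that drifts along the Z axis and reacts to colliding with the player.
; BeginPlay applies a velocity-change impulse of Speed and picks one of four asteroid sprites at random.
; Tick wraps it back to MaxZ once it falls below MinZ.
; On hit, actors tagged Player trigger an explosion emitter and debug print, while others only print.
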(event EventBeginPlay
  (Physics|AddImpulse (Variables|Default|GetCapsule) (Math|Vector|MakeVector 0.0 0.0 (Variables|Default|GetSpeed)) "None" true)
  (switch int (Math|Random|RandomInteger 4)
    (:0
      (Rendering|Components|Sprite|SetSprite (Variables|Default|GetPaperSprite) "/Game/Assets/Obstacles/Asteroids_Asteroid_0.Asteroids_Asteroid_0"))
    (:1
      (Rendering|Components|Sprite|SetSprite (Variables|Default|GetPaperSprite) "/Game/Assets/Obstacles/Asteroids_Asteroid_1.Asteroids_Asteroid_1"))
    (:2
      (Rendering|Components|Sprite|SetSprite (Variables|Default|GetPaperSprite) "/Game/Assets/Obstacles/Asteroids_Asteroid_2.Asteroids_Asteroid_2"))
    (:3
      (Rendering|Components|Sprite|SetSprite (Variables|Default|GetPaperSprite) "/Game/Assets/Obstacles/Asteroids_Asteroid_3.Asteroids_Asteroid_3"))))

(event Collision|EventActorBeginOverlap
  (params (OtherActor :type Actor%20Object%20Reference)))

(event EventTick
  (params (DeltaSeconds :type Float%20%28single-precision%29))
  (bind _returnvalue (Transformation|GetActorLocation))
  (bind (_x _y _z) (Math|Vector|BreakVector _returnvalue))
  (if (< _z (Variables|Default|GetMin%20Z))
    (Transformation|SetActorLocation (Math|Vector|MakeVector _x _y (Variables|Default|GetMax%20Z)) false false)))

(event Collision|EventHit
  (params (MyComp :type Primitive%20Component%20Object%20Reference) (Other :type Actor%20Object%20Reference) (OtherComp :type Primitive%20Component%20Object%20Reference) (bSelfMoved :type Boolean) (HitLocation :type Vector :default "0, 0, 0") (HitNormal :type Vector :default "0, 0, 0") (NormalImpulse :type Vector :default "0, 0, 0") (Hit :type Hit%20Result%20Structure%20%28by%20ref%29))
  (if (Actor|ActorHasTag Other "Player")
    (Utilities|FlowControl|Sequence
      (:then_0
        (Effects|SpawnEmitteratLocation "/Game/2DBullshit/StarterContent/Particles/P_Explosion.P_Explosion" "0, 0, 0"))
      (:then_1
        _))
    (Development|PrintString "Player Collided With Asteroid")
    (else
      (Development|PrintString "Something collided with Asteroid, but not player"))))

(fn ConstructionScript)