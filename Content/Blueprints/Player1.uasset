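; Player1 is a physics-driven actor with four directional thrusters (left, right, up, down) toggled through the CallP2 event.
; BeginPlay applies a one-off, mass-independent torque to the capsule around its Y axis.
; CallP2 branches on its input value to activate a thruster with an attached P_Sparks emitter, or deactivate that thruster and its sparks.
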(event EventCallP2
  (params (value :type Key%20Structure))
  (bind _leftthruster (Variables|Default|GetLeftThruster))
  (bind _downthruster (Variables|Default|GetDownThruster))
  (bind _rightthruster (Variables|Default|GetRightThruster))
  (bind _upthruster (Variables|Default|GetUpThruster))
  (if (== value "Left")
    (Components|Activation|Activate _leftthruster false)
    (bind _returnvalue (Effects|SpawnEmitterAttached "/Game/2DBullshit/StarterContent/Particles/P_Sparks.P_Sparks" _leftthruster "None"))
    (elif (== value "One")
      (Components|Activation|Deactivate _leftthruster)
      (Components|Activation|Deactivate _returnvalue)
      (elif (== value "Down")
        (Components|Activation|Activate _downthruster false)
        (bind _returnvalue_2 (Effects|SpawnEmitterAttached "/Game/2DBullshit/StarterContent/Particles/P_Sparks.P_Sparks" _downthruster "None"))
        (elif (== value "Three")
          (Components|Activation|Deactivate _downthruster)
          (Components|Activation|Deactivate _returnvalue_2)
          (elif (== value "Right")
            (Components|Activation|Activate _rightthruster false)
            (bind _returnvalue_3 (Effects|SpawnEmitterAttached "/Game/2DBullshit/StarterContent/Particles/P_Sparks.P_Sparks" _rightthruster "None"))
            (elif (== value "Two")
              (Components|Activation|Deactivate _rightthruster)
              (Components|Activation|Deactivate _returnvalue_3)
              (elif (== value "Up")
                (Components|Activation|Activate _upthruster false)
                (bind _returnvalue_4 (Effects|SpawnEmitterAttached "/Game/2DBullshit/StarterContent/Particles/P_Sparks.P_Sparks" _upthruster "None"))
                (elif (== value "Four")
                  (Components|Activation|Deactivate _upthruster)
                  (Components|Activation|Deactivate _returnvalue_4))))))))))

(event EventBeginPlay
  ;[1 1 1] Begin Play
  (Class|PrimitiveComponent|AddTorqueinDegrees (Variables|Default|GetCapsule) "0.000000,-3000.000000,0.000000" "None" true))

(fn ConstructionScript)