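; Camera actor Blueprint that follows player 0's pawn in the X-Z plane within set bounds, as in a side-on view.
; Each Tick it clamps the pawn's X and Z between MinX/MaxX and MinZ/MaxZ, holding Y at a fixed depth.
; It teleports straight to that location without sweep or smoothing, and never changes its rotation.
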(event EventBeginPlay)

(event Collision|EventActorBeginOverlap
  (params (OtherActor :type Actor%20Object%20Reference)))

(event EventTick
  (params (DeltaSeconds :type Float%20%28single-precision%29))
  (bind _returnvalue (Game|Player|GetPlayerPawn 0))
  (bind _returnvalue_2 (Transformation|GetActorLocation _returnvalue))
  (bind (_x _y _z) (Math|Vector|BreakVector _returnvalue_2))
  (Transformation|SetActorLocation (Math|Vector|MakeVector (Math|Float|Min(Float) (Math|Float|Max(Float) (Variables|Default|GetMin%20X) _x) (Variables|Default|GetMax%20X)) 1e+03 (Math|Float|Min(Float) (Math|Float|Max(Float) (Variables|Default|GetMin%20Z) _z) (Variables|Default|GetMax%20Z))) false true))

(fn ConstructionScript)