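; Player-one cat pawn, a spinning physics sphere with a sprite, steered by four directional thrusters among asteroids.
; Input actions toggle each thruster along with an attached spark emitter.
; Hitting an "Enemy"-tagged actor explodes and hides the cat, removes the player, and shows the FailMenu after a delay.
; It also relays a second set of keyboard direction inputs to CatPawn2 through CallP2, found via GetAllActorsOfClass.
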(event Custom|GoToFailScreen
  (bind _returnvalue (Game|GetPlayerController 0))
  ;[1 1 1] Collision With Asteroid
  (bind _returnvalue_2 (UserInterface|CreateWidget "/Game/UI/FailMenu.FailMenu_C" _returnvalue))
  (UserInterface|Viewport|AddtoViewport _returnvalue_2 0)
  (bind _output_get (Variables|/Script/Engine.PlayerController|SetbShowMouseCursor _returnvalue true))
  (Input|SetInputModeGameandUI _returnvalue _returnvalue_2 "DoNotLock" _output_get))

(event EventBeginPlay
  ;[1 1 1] Begin Play
  (Class|PrimitiveComponent|AddTorqueinDegrees (Variables|Default|GetSphere) "0.000000,3000.000000,0.000000" "None" true)
  (Variables|Default|SetCatIsDead false))

(event Collision|EventHit
  (params (MyComp :type Primitive%20Component%20Object%20Reference) (Other :type Actor%20Object%20Reference) (OtherComp :type Primitive%20Component%20Object%20Reference) (bSelfMoved :type Boolean) (HitLocation :type Vector :default "0, 0, 0") (HitNormal :type Vector :default "0, 0, 0") (NormalImpulse :type Vector :default "0, 0, 0") (Hit :type Hit%20Result%20Structure%20%28by%20ref%29))
  ;[1 1 1] Collision With Asteroid
  (if (Actor|ActorHasTag Other "Enemy")
    (if (not (Variables|Default|GetCatIsDead))
      (Input|DisableInput 0)
      (Effects|SpawnEmitteratLocation "/Game/Particles/P_Explosion.P_Explosion" (Transformation|GetWorldLocation (Variables|Default|GetSphere)))
      (Class|GameplayStatics|RemovePlayer 0 true)
      (Rendering|SetVisibility (Variables|Default|GetPaperSprite) false false)
      (Utilities|Time|SetTimerbyEvent (delegate Custom|GoToFailScreen) 2.0)
      (Variables|Default|SetCatIsDead true))))

(event Input|ActionEvents|InputActionKeyboarddown
  (params (Key :type Key%20Structure :default "None"))
  (:Pressed
    (bind _outactors (Actor|GetAllActorsOfClass "/Game/Blueprints/CatPawn2.CatPawn2_C"))
    (Default|CallP2 _outactors "Down"))
  (:Released
    (bind _outactors_2 (Actor|GetAllActorsOfClass "/Game/Blueprints/CatPawn2.CatPawn2_C"))
    (Default|CallP2 _outactors_2 "Three")))

(event Input|ActionEvents|InputActionKeyboardup
  (params (Key :type Key%20Structure :default "None"))
  (:Pressed
    (bind _outactors (Actor|GetAllActorsOfClass "/Game/Blueprints/CatPawn2.CatPawn2_C"))
    (Default|CallP2 _outactors "Up"))
  (:Released
    (bind _outactors_2 (Actor|GetAllActorsOfClass "/Game/Blueprints/CatPawn2.CatPawn2_C"))
    (Default|CallP2 _outactors_2 "Four")))

(event Input|ActionEvents|InputActiondown
  (params (Key :type Key%20Structure :default "None"))
  (bind _downthruster (Variables|Default|GetDownThruster))
  ;[1 1 1] Down Thruster Input
  (:Pressed
    (Components|Activation|Activate _downthruster false)
    (bind _returnvalue (Effects|SpawnEmitterAttached "/Game/Particles/P_Sparks.P_Sparks" _downthruster "None")))
  (:Released
    (Components|Activation|Deactivate _downthruster)
    (Components|Activation|Deactivate _returnvalue)))

(event Input|ActionEvents|InputActionup
  (params (Key :type Key%20Structure :default "None"))
  (bind _upthruster (Variables|Default|GetUpThruster))
  ;[1 1 1] Top Thruster Input
  (:Pressed
    (Components|Activation|Activate _upthruster false)
    (bind _returnvalue (Effects|SpawnEmitterAttached "/Game/Particles/P_Sparks.P_Sparks" _upthruster "None")))
  (:Released
    (Components|Activation|Deactivate _upthruster)
    (Components|Activation|Deactivate _returnvalue)))

(event Input|ActionEvents|InputActionright
  (params (Key :type Key%20Structure :default "None"))
  (bind _rightthruster (Variables|Default|GetRightThruster))
  ;[1 1 1] Right Thruster Input
  (:Pressed
    (Components|Activation|Activate _rightthruster false)
    (bind _returnvalue (Effects|SpawnEmitterAttached "/Game/Particles/P_Sparks.P_Sparks" _rightthruster "None")))
  (:Released
    (Components|Activation|Deactivate _rightthruster)
    (Components|Activation|Deactivate _returnvalue)))

(event Input|ActionEvents|InputActionleft
  (params (Key :type Key%20Structure :default "None"))
  (bind _leftthruster (Variables|Default|GetLeftThruster))
  ;[1 1 1] Left Thruster Input
  (:Pressed
    (Components|Activation|Activate _leftthruster false)
    (bind _returnvalue (Effects|SpawnEmitterAttached "/Game/Particles/P_Sparks.P_Sparks" _leftthruster "None")))
  (:Released
    (Components|Activation|Deactivate _leftthruster)
    (Components|Activation|Deactivate _returnvalue)))

(event Input|ActionEvents|InputActionKeyboardleft
  (params (Key :type Key%20Structure :default "None"))
  (:Pressed
    (bind _outactors (Actor|GetAllActorsOfClass "/Game/Blueprints/CatPawn2.CatPawn2_C"))
    (Default|CallP2 _outactors "Left"))
  (:Released
    (bind _outactors_2 (Actor|GetAllActorsOfClass "/Game/Blueprints/CatPawn2.CatPawn2_C"))
    (Default|CallP2 _outactors_2 "One")))

(event Input|ActionEvents|InputActionKeyboardright
  (params (Key :type Key%20Structure :default "None"))
  (:Pressed
    (bind _outactors (Actor|GetAllActorsOfClass "/Game/Blueprints/CatPawn2.CatPawn2_C"))
    (Default|CallP2 _outactors "Right"))
  (:Released
    (bind _outactors_2 (Actor|GetAllActorsOfClass "/Game/Blueprints/CatPawn2.CatPawn2_C"))
    (Default|CallP2 _outactors_2 "Two")))

(fn ConstructionScript)