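; Player 0 pawn for what appears to be local two-player play, moved by four directional thrusters and given an initial torque on its capsule at BeginPlay.
; Its directional inputs activate the matching thruster and attach a spark emitter, deactivating both on release.
; It also receives the separate Keyboard directional actions and relays presses and releases to Player1 actors through CallP2, so this pawn handles input for both players.
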(event EventBeginPlay
  ;[1 1 1] Begin Play
  (Class|PrimitiveComponent|AddTorqueinDegrees (Variables|Default|GetCapsule) "0.000000,3000.000000,0.000000" "None" true))

(event Input|ActionEvents|InputActionKeyboarddown
  (params (Key :type Key%20Structure :default "None"))
  (:Pressed
    (bind _outactors (Actor|GetAllActorsOfClass "/Game/Blueprints/Player1.Player1_C"))
    (Default|CallP2 _outactors "Down"))
  (:Released
    (bind _outactors_2 (Actor|GetAllActorsOfClass "/Game/Blueprints/Player1.Player1_C"))
    (Default|CallP2 _outactors_2 "Three")))

(event Input|ActionEvents|InputActionKeyboardup
  (params (Key :type Key%20Structure :default "None"))
  (:Pressed
    (bind _outactors (Actor|GetAllActorsOfClass "/Game/Blueprints/Player1.Player1_C"))
    (Default|CallP2 _outactors "Up"))
  (:Released
    (bind _outactors_2 (Actor|GetAllActorsOfClass "/Game/Blueprints/Player1.Player1_C"))
    (Default|CallP2 _outactors_2 "Four")))

(event Input|ActionEvents|InputActiondown
  (params (Key :type Key%20Structure :default "None"))
  (bind _downthruster (Variables|Default|GetDownThruster))
  ;[1 1 1] Down Thruster Input
  (:Pressed
    (Components|Activation|Activate _downthruster false)
    (bind _returnvalue (Effects|SpawnEmitterAttached "/Game/2DBullshit/StarterContent/Particles/P_Sparks.P_Sparks" _downthruster "None")))
  (:Released
    (Components|Activation|Deactivate _downthruster)
    (Components|Activation|Deactivate _returnvalue)))

(event Input|ActionEvents|InputActionup
  (params (Key :type Key%20Structure :default "None"))
  (bind _upthruster (Variables|Default|GetUpThruster))
  ;[1 1 1] Top Thruster Input
  (:Pressed
    (Components|Activation|Activate _upthruster false)
    (bind _returnvalue (Effects|SpawnEmitterAttached "/Game/2DBullshit/StarterContent/Particles/P_Sparks.P_Sparks" _upthruster "None")))
  (:Released
    (Components|Activation|Deactivate _upthruster)
    (Components|Activation|Deactivate _returnvalue)))

(event Input|ActionEvents|InputActionright
  (params (Key :type Key%20Structure :default "None"))
  (bind _rightthruster (Variables|Default|GetRightThruster))
  ;[1 1 1] Right Thruster Input
  (:Pressed
    (Components|Activation|Activate _rightthruster false)
    (bind _returnvalue (Effects|SpawnEmitterAttached "/Game/2DBullshit/StarterContent/Particles/P_Sparks.P_Sparks" _rightthruster "None")))
  (:Released
    (Components|Activation|Deactivate _rightthruster)
    (Components|Activation|Deactivate _returnvalue)))

(event Input|ActionEvents|InputActionleft
  (params (Key :type Key%20Structure :default "None"))
  (bind _leftthruster (Variables|Default|GetLeftThruster))
  ;[1 1 1] Left Thruster Input
  (:Pressed
    (Components|Activation|Activate _leftthruster false)
    (bind _returnvalue (Effects|SpawnEmitterAttached "/Game/2DBullshit/StarterContent/Particles/P_Sparks.P_Sparks" _leftthruster "None")))
  (:Released
    (Components|Activation|Deactivate _leftthruster)
    (Components|Activation|Deactivate _returnvalue)))

(event Input|ActionEvents|InputActionKeyboardleft
  (params (Key :type Key%20Structure :default "None"))
  (:Pressed
    (bind _outactors (Actor|GetAllActorsOfClass "/Game/Blueprints/Player1.Player1_C"))
    (Default|CallP2 _outactors "Left"))
  (:Released
    (bind _outactors_2 (Actor|GetAllActorsOfClass "/Game/Blueprints/Player1.Player1_C"))
    (Default|CallP2 _outactors_2 "One")))

(event Input|ActionEvents|InputActionKeyboardright
  (params (Key :type Key%20Structure :default "None"))
  (:Pressed
    (bind _outactors (Actor|GetAllActorsOfClass "/Game/Blueprints/Player1.Player1_C"))
    (Default|CallP2 _outactors "Right"))
  (:Released
    (bind _outactors_2 (Actor|GetAllActorsOfClass "/Game/Blueprints/Player1.Player1_C"))
    (Default|CallP2 _outactors_2 "Two")))

(fn ConstructionScript)

(fn NewFunction0)