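; CatPawn2 is a pawn steered by four directional thrusters, driven through a CallP2 event.
; BeginPlay gives the Sphere an initial spin and starts a looping timer for CheckSpin, which is not defined here.
; CallP2 decodes one value to switch each thruster on or off, along with its attached sparks and a jet sound.
; The jet sounds play at the world origin rather than at the pawn.
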(event EventCallP2
  (params (value :type Key%20Structure :default "None"))
  (bind _leftthruster (Variables|Default|GetLeftThruster))
  (bind _downthruster (Variables|Default|GetDownThruster))
  (bind _rightthruster (Variables|Default|GetRightThruster))
  (bind _upthruster (Variables|Default|GetUpThruster))
  (if (== value "Left")
    (Components|Activation|Activate _leftthruster false)
    (bind _returnvalue (Effects|SpawnEmitterAttached "/Game/Particles/P_Sparks.P_Sparks" _leftthruster "None"))
    (bind _returnvalue_2 (Audio|SpawnSoundatLocation "/Game/Assets/Audio/CS_JetSound_Cue.CS_JetSound_Cue" "0, 0, 0" "0, 0, 0" 1.0 1.0 0.0 0 0))
    (elif (== value "One")
      (Components|Activation|Deactivate _leftthruster)
      (Components|Activation|Deactivate _returnvalue)
      (Components|Activation|Deactivate _returnvalue_2)
      (elif (== value "Down")
        (Components|Activation|Activate _downthruster false)
        (bind _returnvalue_3 (Effects|SpawnEmitterAttached "/Game/Particles/P_Sparks.P_Sparks" _downthruster "None"))
        (bind _returnvalue_4 (Audio|SpawnSoundatLocation "/Game/Assets/Audio/CS_JetSound_Cue.CS_JetSound_Cue" "0, 0, 0" "0, 0, 0" 1.0 1.0 0.0 0 0))
        (elif (== value "Three")
          (Components|Activation|Deactivate _downthruster)
          (Components|Activation|Deactivate _returnvalue_3)
          (Components|Activation|Deactivate _returnvalue_4)
          (elif (== value "Right")
            (Components|Activation|Activate _rightthruster false)
            (bind _returnvalue_5 (Effects|SpawnEmitterAttached "/Game/Particles/P_Sparks.P_Sparks" _rightthruster "None"))
            (bind _returnvalue_6 (Audio|SpawnSoundatLocation "/Game/Assets/Audio/CS_JetSound_Cue.CS_JetSound_Cue" "0, 0, 0" "0, 0, 0" 1.0 1.0 0.0 0 0))
            (elif (== value "Two")
              (Components|Activation|Deactivate _rightthruster)
              (Components|Activation|Deactivate _returnvalue_5)
              (Components|Activation|Deactivate _returnvalue_6)
              (elif (== value "Up")
                (Components|Activation|Activate _upthruster false)
                (bind _returnvalue_7 (Effects|SpawnEmitterAttached "/Game/Particles/P_Sparks.P_Sparks" _upthruster "None"))
                (bind _returnvalue_8 (Audio|SpawnSoundatLocation "/Game/Assets/Audio/CS_JetSound_Cue.CS_JetSound_Cue" "0, 0, 0" "0, 0, 0" 1.0 1.0 0.0 0 0))
                (elif (== value "Four")
                  (Components|Activation|Deactivate _upthruster)
                  (Components|Activation|Deactivate _returnvalue_7)
                  (Components|Activation|Deactivate _returnvalue_8))))))))))

(event EventBeginPlay
  ;[1 1 1] Begin Play
  (Class|PrimitiveComponent|AddTorqueinDegrees (Variables|Default|GetSphere) "0.000000,-3000.000000,0.000000" "None" true)
  (Utilities|Time|SetTimerbyFunctionName 0 "CheckSpin" 0.7 true))

(fn ConstructionScript
  (|CallParentFunction))